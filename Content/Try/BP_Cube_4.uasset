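; BP_Cube_4 is an actor whose static mesh hangs frozen at level start, then turns into a falling physics object.
; BeginPlay disables physics simulation and gravity on the mesh, waits a random delay of roughly ten seconds, then enables both.
; All logic sits in that single event chain, and the construction script is empty.
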(event `self.ReceiveBeginPlay`
  (`PrimitiveComponent.SetSimulatePhysics` (`self.StaticMeshComponent`) false)
  (`PrimitiveComponent.SetEnableGravity` (`self.StaticMeshComponent`) false)
  (bind _output_get (set `self.Time` (`KismetMathLibrary.RandomFloatInRange` 9.0 11.0)))
  (`KismetSystemLibrary.Delay` _output_get)
  (`PrimitiveComponent.SetSimulatePhysics` (`self.StaticMeshComponent`) true)
  (`PrimitiveComponent.SetEnableGravity` (`self.StaticMeshComponent`) true))

(fn `UserConstructionScript`)